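; Parent ability actor for a tile-based, turn-based game: equips to the current pawn's hotbar and targets self, allies or enemies.
; InitiateAbility checks resources and highlights tiles through Grid_Manager; a click validates faction and range.
; Execution turns the sprite, optionally plays a melee lunge timeline, rolls dodge, applies weapon damage, frames ranged hits and advances the turn.
; Costs are unfinished: health, MP and FP are set to zero on use.
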(event `self.ReceiveBeginPlay`
  ;[1 1 1] References
  (bind _outactors (`GameplayStatics.GetAllActorsOfClass` "/Game/TileBased/Blueprints/Gameplay/TB_GameMode.TB_GameMode_C"))
  (set `self.TBGameMode_Ref` (`KismetArrayLibrary.Array_Get` _outactors))
  (bind _outactors_2 (`GameplayStatics.GetAllActorsOfClass` "/Game/TileBased/Blueprints/Gameplay/Grid_Manager.Grid_Manager_C"))
  (set `self.GridManager_Ref` (`KismetArrayLibrary.Array_Get` _outactors_2))
  (bind _outactors_3 (`GameplayStatics.GetAllActorsOfClass` "/Game/TileBased/Blueprints/Gameplay/Grid_Camera.Grid_Camera_C"))
  (set `self.GridCamera_Ref` (`KismetArrayLibrary.Array_Get` _outactors_3)))

(event `EquipAbility`
  ;[1 1 1] Event Equip Ability (on hotbar)
  (`KismetArrayLibrary.Array_Add` (`/Game/TileBased/Blueprints/Pawns/Unit.HotbarStruct` (`/Game/TileBased/Blueprints/Gameplay/TB_GameMode.CurrentPawn` (`self.TBGameMode_Ref`))) self))

(event `Initiate Ability`
  (bind _gridmanager_ref (`self.GridManager_Ref`))
  (bind _range (`self.Range`))
  (bind _tbgamemode_ref (`self.TBGameMode_Ref`))
  (bind _range_2 (`self.Range`))
  (bind _gridmanager_ref_2 (`self.GridManager_Ref`))
  (bind _currentpawn (`/Game/TileBased/Blueprints/Gameplay/TB_GameMode.CurrentPawn` _tbgamemode_ref))
  ;[1 1 1] Initiate Ability
  (if (`/Game/TileBased/Blueprints/Gameplay/TB_GameMode.PlayerTurn` _tbgamemode_ref)
    ;;[1 1 1] Enough AP?
    (if (>= (`/Game/TileBased/Blueprints/Pawns/Unit.APReg_Current` _currentpawn) (`KismetMathLibrary.FTrunc` (`self.APCost`)))
      ;;[1 1 1] Enough Health?
      (if (>= (`/Game/TileBased/Blueprints/Pawns/Unit.CurrentHealth` _currentpawn) (`self.HPCost`))
        ;;[1 1 1] Enough Health?
        (if (>= (`/Game/TileBased/Blueprints/Pawns/Unit.MaxMana` _currentpawn) (`self.ManaCost`))
          ;;[1 1 1] Enough AP?
          (if (>= (`/Game/TileBased/Blueprints/Pawns/Unit.MaxFinesse` _currentpawn) (`self.FinesseCost`))
            (`self.EnableInput` (`GameplayStatics.GetPlayerController` 0))
            ;;[1 1 1] Clear Markers
            (`/Game/TileBased/Blueprints/Gameplay/Grid_Manager.Clear all in range mesh markers` _gridmanager_ref_2)
            (`KismetArrayLibrary.Array_Clear` (`/Game/TileBased/Blueprints/Gameplay/Grid_Manager.CanMoveToArray` _gridmanager_ref_2))
            (`|ExecutionSequence`
              (:`then_0`
                ;;[1 1 1] Can target Self -> Set min range
                (if (`self.TargetSelf`)
                  (set `self.MinRange_Temp` 0)
                  ;;[1 1 1] Can target Ally?
                  (if (`self.TargetAlly`)
                    ;;[1 1 1] Find tiles with viable allied targets
                    (`/Game/TileBased/Blueprints/Gameplay/Grid_Manager.Find Tiles In Range` _gridmanager_ref (`/Game/TileBased/Blueprints/Pawns/Unit.Index` _currentpawn) _range true true true "NewEnumerator0" true (* _range (/ (+ (`/Game/TileBased/Blueprints/Gameplay/Grid_Manager.TileBoundsX` _gridmanager_ref) (`/Game/TileBased/Blueprints/Gameplay/Grid_Manager.TileBoundsY` _gridmanager_ref)) 2.0)) (`self.MinRange_Temp`) false :!label _label)
                    (else
                      (`self.Target self only`)))
                  (else
                    (set `self.MinRange_Temp` 1)
                    (if (`self.TargetAlly`)
                      (goto _label)))))
              (:`then_1`
                ;;[1 1 1] Find tiles with viable enemy target
                (if (`self.TargetEnemy`)
                  (`/Game/TileBased/Blueprints/Gameplay/Grid_Manager.Find Tiles In Range` _gridmanager_ref (`/Game/TileBased/Blueprints/Pawns/Unit.Index` _currentpawn) _range_2 true true true "NewEnumerator1" true (* _range_2 (/ (+ (`/Game/TileBased/Blueprints/Gameplay/Grid_Manager.TileBoundsX` _gridmanager_ref) (`/Game/TileBased/Blueprints/Gameplay/Grid_Manager.TileBoundsY` _gridmanager_ref)) 2.0)) 1 false))))
            (else
              (`KismetSystemLibrary.PrintString` "Not enough AP")))
          (else
            (`KismetSystemLibrary.PrintString` "Not enough MP")))
        (else
          (`KismetSystemLibrary.PrintString` "Not enough HP")))
      (else
        (`KismetSystemLibrary.PrintString` "Not enough AP")))))

(event `Target self only`
  (bind _gridmanager_ref (`self.GridManager_Ref`))
  (bind _gridmanager_ref_2 (`self.GridManager_Ref`))
  (bind _targetmarker (`/Game/TileBased/Blueprints/Gameplay/Grid_Manager.TargetMarker` _gridmanager_ref_2))
  (bind _currentpawn (`/Game/TileBased/Blueprints/Gameplay/TB_GameMode.CurrentPawn` (`self.TBGameMode_Ref`)))
  (bind _currentpawn_2 (`/Game/TileBased/Blueprints/Gameplay/TB_GameMode.CurrentPawn` (`self.TBGameMode_Ref`)))
  (bind _currentpawn_3 (`/Game/TileBased/Blueprints/Gameplay/TB_GameMode.CurrentPawn` (`self.TBGameMode_Ref`)))
  (bind _currentpawn_4 (`/Game/TileBased/Blueprints/Gameplay/TB_GameMode.CurrentPawn` (`self.TBGameMode_Ref`)))
  (bind _item (`KismetArrayLibrary.Array_Get` (`/Game/TileBased/Blueprints/Gameplay/Grid_Manager.Pawn Array` (`self.GridManager_Ref`)) (`self.Clicked Tile`)))
  (bind (_returnvalue_roll _returnvalue_pitch) (`KismetMathLibrary.BreakRotator` (`self.K2_GetActorRotation` _currentpawn)))
  (bind _returnvalue_x (`KismetMathLibrary.BreakVector` (`self.K2_GetActorLocation` _currentpawn)))
  (bind _returnvalue (`self.K2_GetActorLocation` _currentpawn_3))
  (bind _spriteanchor (`/Game/TileBased/Blueprints/Pawns/Unit.SpriteAnchor` _currentpawn))
  (bind (_returnvalue_roll_2 _returnvalue_pitch_2 _returnvalue_yaw) (`KismetMathLibrary.BreakRotator` (`SceneComponent.K2_GetComponentRotation` _spriteanchor)))
  ;[1 1 1] Is the clicked tile a viable target?
  ;[1 1 1] Mesh and Spline CleanUp
  (`/Game/TileBased/Blueprints/Gameplay/Grid_Manager.Clear all in range mesh markers` _gridmanager_ref :!label _label_2)
  (`/Game/TileBased/Blueprints/Gameplay/Grid_Manager.Destroy and clear spline path` _gridmanager_ref)
  ;[1 1 1] Target marker
  (`/Game/TileBased/Blueprints/Gameplay/Grid_Manager.Set Marker Location` (`self.GridManager_Ref`) (0.0 0.0 0.0) true (`/Game/TileBased/Blueprints/Pawns/Unit.Index` _item) (`/Game/TileBased/Blueprints/Gameplay/Grid_Manager.Target Marker Decal` _gridmanager_ref_2) _targetmarker) ; Set target marker location to victim location
  (`/Game/TileBased/Blueprints/Gameplay/Grid_Manager.Set Marker Visibility` (`self.GridManager_Ref`) true _targetmarker)
  ;[1 1 1] Sprite Rotation (Create function --> same at unit parent!!!)
  (bind _output_get (set `/Game/TileBased/Blueprints/Pawns/Unit.Target Location` (`self.K2_GetActorLocation` _item) _currentpawn))
  (bind _returnvalue_2 (`KismetMathLibrary.FTrunc` (- _returnvalue_x (.x _output_get))))
  (`SceneComponent.K2_SetWorldRotation` _spriteanchor (`KismetMathLibrary.MakeRotator` _returnvalue_roll _returnvalue_pitch (`KismetMathLibrary.SelectFloat` _returnvalue_yaw (`KismetMathLibrary.SelectFloat` 0.0 180.0 (> _returnvalue_2 0)) (== _returnvalue_2 0))) false false)
  ;[1 1 1] Resource cost
  (set `/Game/TileBased/Blueprints/Pawns/Unit.CurrentAP` (- (`/Game/TileBased/Blueprints/Pawns/Unit.CurrentAP` _currentpawn_2) (`self.APCost`)) _currentpawn_2)
  (set `/Game/TileBased/Blueprints/Pawns/Unit.CurrentHealth` 0.0 _currentpawn_2)
  (set `/Game/TileBased/Blueprints/Pawns/Unit.CurrentMP` 0.0 _currentpawn_2)
  (set `/Game/TileBased/Blueprints/Pawns/Unit.CurrentFP` 0.0 _currentpawn_2)
  (`GameplayStatics.PlaySound2D` (`self.HitSound`))
  (if (`/Game/TileBased/Blueprints/Pawns/Unit.Melee Attack Animation` _currentpawn_3)
    ;[1 1 1] Melee attack animation
    (bind (_direction _attack_timeline) (`Timeline|Timeline_1` :!via `PlayFromStart`)
      (:`Update`
        (`self.K2_SetActorLocation` (+ (* (- (`self.K2_GetActorLocation` _item) _returnvalue) _attack_timeline) _returnvalue)))
      (:`Attack Hit`
        (if (`self.CanBeDodge`) :!label _label_3
          ;[1 1 1] Dodge
          (if (> (+ (`KismetMathLibrary.RandomInteger` 100) 1) (`/Game/TileBased/Blueprints/Pawns/Unit.%Dodge_Current` _item))
            (if (`self.WeaponDamage`) :!label _label_4
              (`/Game/TileBased/Blueprints/Pawns/Unit.Receive Damage` _item (`/Game/TileBased/Blueprints/Pawns/Unit.Damage` _currentpawn_4) (`/Game/TileBased/Blueprints/Pawns/Unit.Anim Damage Delay` _currentpawn_4))
              (`self.FinishAbilityUse` _item))
            (else
              (`KismetSystemLibrary.PrintString` "Dodge")
              (`/Game/TileBased/Blueprints/Pawns/Unit.Receive Damage` _item 0.0 (`/Game/TileBased/Blueprints/Pawns/Unit.Anim Damage Delay` (`/Game/TileBased/Blueprints/Gameplay/TB_GameMode.CurrentPawn` (`self.TBGameMode_Ref`))))
              (`self.FinishAbilityUse` _item)))
          (else
            (goto _label_4)))))
    (else
      (goto _label_3))))

(event `InputAction|Click`
  (params (Key :type "Key Structure" :default "AnyKey"))
  (bind _gridmanager_ref (`self.GridManager_Ref`))
  (:`Pressed`
    ;[1 1 1] Get Hit Location, Index and check if and what pawn is on the tile
    (bind (_index _location _tracehit) (`/Game/TileBased/Blueprints/Gameplay/Grid_Manager.Get hit tile location and index` _gridmanager_ref))
    (if _tracehit
      (set `self.Clicked Tile` _index)
      ;[1 1 1] Is the clicked tile a viable target?
      (switch `/Game/TileBased/Blueprints/Gameplay/Enums/Enum_Faction` (`/Game/TileBased/Blueprints/Pawns/Unit.Faction` (`KismetArrayLibrary.Array_Get` (`/Game/TileBased/Blueprints/Gameplay/Grid_Manager.Pawn Array` _gridmanager_ref) _index)) ; What pawn is on the clicked tile?
        (:`NewEnumerator0`
          (if (`self.TargetAlly`)
            (if (`self.TargetSelf`)
              ;;[1 1 1] Does clicked actor equal self
              (if (== (`/Game/TileBased/Blueprints/Gameplay/TB_GameMode.CurrentPawn` (`self.TBGameMode_Ref`)) (`KismetArrayLibrary.Array_Get` (`/Game/TileBased/Blueprints/Gameplay/Grid_Manager.Pawn Array` (`self.GridManager_Ref`)) (`self.Clicked Tile`)))
                (goto _label_2)
                (else
                  _)))
            (if (> (`KismetArrayLibrary.Array_Get` (`/Game/TileBased/Blueprints/Gameplay/Grid_Manager.RangeArray` (`self.GridManager_Ref`)) (`self.Clicked Tile`)) 0) :!label _label_5
              (goto _label_2))))
        (:`NewEnumerator1`
          (if (`self.TargetEnemy`)
            (goto _label_5)))))))

(fn `FinishAbilityUse`
  (params (Victim :type "/Game/TileBased/Blueprints/Pawns/Unit Object Reference"))
  (bind _gridcamera_ref (`self.GridCamera_Ref`))
  (bind _currentpawn (`/Game/TileBased/Blueprints/Gameplay/TB_GameMode.CurrentPawn` (`self.TBGameMode_Ref`)))
  (if (> (`/Game/TileBased/Blueprints/Gameplay/Grid_Manager.Find Distance (in Tiles) Between Indexes` (`self.GridManager_Ref`) (`/Game/TileBased/Blueprints/Pawns/Unit.Index` _currentpawn) (`/Game/TileBased/Blueprints/Pawns/Unit.Index` Victim)) 1)
    (set `/Game/TileBased/Blueprints/Gameplay/Grid_Camera.CustomTarget` (/ (+ (`self.K2_GetActorLocation` _currentpawn) (`self.K2_GetActorLocation` Victim)) 2) _gridcamera_ref)
    (set `/Game/TileBased/Blueprints/Gameplay/Grid_Camera.Follow Custom Target` true _gridcamera_ref))
  (`/Game/TileBased/Blueprints/Gameplay/TB_GameMode.ChooseNextPawn` (`self.TBGameMode_Ref`) 1.5))

(fn `UserConstructionScript`)